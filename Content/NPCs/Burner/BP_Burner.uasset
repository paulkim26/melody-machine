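; BP_Burner is an NPC that damages the player with a pulsing fire aura while alive.
; Tick drives a Delay that flips MagicAttack about every second, showing the particle system during the attack phase and hiding it otherwise.
; During that phase, each tick has a weighted random chance to spawn fire at its location and damages BP_Player whenever the player is within MagicRadius.
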(event EventBeginPlay
  (|CallParentFunction) ; This node is disabled and will not be called.\nDrag off pins to build functionality.
)

(event Collision|EventActorBeginOverlap
  (params (OtherActor :type Actor%20Object%20Reference))
  (|CallParentFunction OtherActor) ; This node is disabled and will not be called.\nDrag off pins to build functionality.
)

(event EventTick
  (params (DeltaSeconds :type Float%20%28single-precision%29))
  (|CallParentFunction DeltaSeconds)
  (if (Variables|Default|GetAlive)
    (Utilities|FlowControl|Sequence
      (:then_0
        (Utilities|FlowControl|Delay 1.0)
        (Variables|Default|SetMagicAttack (not (Variables|Default|GetMagicAttack))))
      (:then_1
        (if (Variables|Default|GetMagicAttack)
          (Utilities|FlowControl|Sequence
            (:then_0
              (Rendering|SetVisibility (Variables|Default|GetParticleSystem) true false)
              (if (Math|Random|RandomBoolwithWeight 0.3)
                (Effects|SpawnEmitteratLocation "/Game/StarterContent/Particles/P_Fire.P_Fire" (Transformation|GetActorLocation))))
            (:then_1
              (bind _distance (CallFunction|DistancetoPlayer))
              (if (<= _distance (Variables|Default|GetMagicRadius))
                (bind _asbp_player (Utilities|Casting|CastToBP_Player (Game|Player|GetPlayerPawn 0)))
                (Default|TakeDamage _asbp_player))))
          (else
            (Rendering|SetVisibility (Variables|Default|GetParticleSystem) false false)))))))

(fn ConstructionScript
  (|CallParentFunction))