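; Moving platform actor that shuttles back and forth between its starting location and the location of a Target actor, pausing at each end.
; Tick steps a PathAlpha by frame delta over TravelSeconds and lerps the actor's position between the two points, without sweep.
; PathState flips the direction at each endpoint and restarts a DelaySeconds countdown, which also holds the platform at BeginPlay before its first move.
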(event EventBeginPlay
  (Variables|Default|SetStartLocation (Transformation|GetActorLocation))
  (CallFunction|InitDelay))

(event EventTick
  (params (DeltaSeconds :type Float%20%28single-precision%29))
  (CallFunction|SetPlatformPosition))

(fn ConstructionScript)

(fn MovetoEnd
  (if (< (+ (Variables|Default|GetPathAlpha) (/ (Utilities|Time|GetWorldDeltaSeconds) (Variables|Default|GetTravelSeconds))) 1.0)
    (Variables|Default|SetPathAlpha (+ (Variables|Default|GetPathAlpha) (/ (Utilities|Time|GetWorldDeltaSeconds) (Variables|Default|GetTravelSeconds))))
    (else
      (Variables|Default|SetPathAlpha 1.0)
      (Variables|Default|SetPathState 1)
      (CallFunction|InitDelay))))

(fn SetPlatformPosition
  (if (== (Variables|Default|GetDelay) 0.0)
    (switch int (Variables|Default|GetPathState)
      (:0
        (CallFunction|MovetoEnd))
      (:1
        (CallFunction|MovetoStart)))
    (Transformation|SetActorLocation (Math|Vector|Lerp(Vector) (Variables|Default|GetStartLocation) (Transformation|GetActorLocation (Variables|Default|GetTarget)) (Variables|Default|GetPathAlpha)) false false)
    (else
      (CallFunction|StepDelay))))

(fn MovetoStart
  (if (> (- (Variables|Default|GetPathAlpha) (/ (Utilities|Time|GetWorldDeltaSeconds) (Variables|Default|GetTravelSeconds))) 0.0)
    (Variables|Default|SetPathAlpha (- (Variables|Default|GetPathAlpha) (/ (Utilities|Time|GetWorldDeltaSeconds) (Variables|Default|GetTravelSeconds))))
    (else
      (Variables|Default|SetPathAlpha 0.0)
      (Variables|Default|SetPathState 0)
      (CallFunction|InitDelay))))

(fn StepDelay
  (if (> (- (Variables|Default|GetDelay) (Utilities|Time|GetWorldDeltaSeconds)) 0.0)
    (Variables|Default|SetDelay (- (Variables|Default|GetDelay) (Utilities|Time|GetWorldDeltaSeconds)))
    (else
      (Variables|Default|SetDelay 0.0))))

(fn InitDelay
  (Variables|Default|SetDelay (Variables|Default|GetDelaySeconds)))