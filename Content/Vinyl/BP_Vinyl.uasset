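; Spinning vinyl record pickup that flies into the player and destroys itself when collected.
; Begin play offsets the yaw based on distance from the world origin to vary each record's rotation, and Tick keeps it spinning.
; Player overlap doubles spin speed and plays one of nine random DJ scratch sounds at the world origin.
; Tick then lerps it from its start location to the player's current position over CollectAnimTime.
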(event EventBeginPlay
  (bind _output_get (Variables|Default|SetStartLocation (Transformation|GetActorLocation)))
  ;[1 1 1] "randomize" initial rotation
  (Transformation|AddActorLocalRotation (Math|Rotator|MakeRotator 0.0 0.0 (/ (Math|Vector|VectorLength _output_get) 5.0)) false false))

(event Collision|EventActorBeginOverlap
  (params (OtherActor :type Actor%20Object%20Reference))
  (if (== OtherActor (Game|GetPlayerCharacter 0))
    (CallFunction|CollectStart)))

(event EventTick
  (params (DeltaSeconds :type Float%20%28single-precision%29))
  (Transformation|AddActorLocalRotation (Math|Rotator|MakeRotator 0.0 0.0 (* DeltaSeconds (Variables|Default|GetSpinSpeed))) false false)
  (CallFunction|CollectStep))

(fn ConstructionScript)

(fn CollectStep
  (if (Variables|Default|GetCollect)
    (bind _output_get (Variables|Default|SetAnimAlpha (+ (/ (Utilities|Time|GetWorldDeltaSeconds) (Variables|Default|GetCollectAnimTime)) (Variables|Default|GetAnimAlpha))))
    (if (< _output_get 1.0)
      (Transformation|SetActorLocation (Math|Vector|Lerp(Vector) (Variables|Default|GetStartLocation) (Transformation|GetActorLocation (Game|GetPlayerCharacter 0)) (Variables|Default|GetAnimAlpha)) false false)
      (else
        (Actor|DestroyActor)))))

(fn CollectStart
  (Variables|Default|SetCollect true)
  (Variables|Default|SetSpinSpeed (* (Variables|Default|GetSpinSpeed) 2.0))
  (switch int (Math|Random|RandomIntegerinRange 1 9)
    (:1
      (Audio|PlaySoundatLocation "/Game/Sounds/dj/dj_scratch_1.dj_scratch_1" "0, 0, 0" "0, 0, 0" 1.0 1.0 0.0 0 0 0))
    (:2
      (Audio|PlaySoundatLocation "/Game/Sounds/dj/dj_scratch_2.dj_scratch_2" "0, 0, 0" "0, 0, 0" 1.0 1.0 0.0 0 0 0))
    (:3
      (Audio|PlaySoundatLocation "/Game/Sounds/dj/dj_scratch_3.dj_scratch_3" "0, 0, 0" "0, 0, 0" 1.0 1.0 0.0 0 0 0))
    (:4
      (Audio|PlaySoundatLocation "/Game/Sounds/dj/dj_scratch_4.dj_scratch_4" "0,0.000000, 0" "0, 0, 0" 1.0 1.0 0.0 0 0 0))
    (:5
      (Audio|PlaySoundatLocation "/Game/Sounds/dj/dj_scratch_5.dj_scratch_5" "0, 0, 0" "0, 0, 0" 1.0 1.0 0.0 0 0 0))
    (:6
      (Audio|PlaySoundatLocation "/Game/Sounds/dj/dj_scratch_6.dj_scratch_6" "0, 0, 0" "0, 0, 0" 1.0 1.0 0.0 0 0 0))
    (:7
      (Audio|PlaySoundatLocation "/Game/Sounds/dj/dj_scratch_7.dj_scratch_7" "0, 0, 0" "0, 0, 0" 1.0 1.0 0.0 0 0 0))
    (:8
      (Audio|PlaySoundatLocation "/Game/Sounds/dj/dj_scratch_8.dj_scratch_8" "0, 0, 0" "0, 0, 0" 1.0 1.0 0.0 0 0 0))
    (:9
      (Audio|PlaySoundatLocation "/Game/Sounds/dj/dj_scratch_9.dj_scratch_9" "0, 0, 0" "0, 0, 0" 1.0 1.0 0.0 0 0 0))))