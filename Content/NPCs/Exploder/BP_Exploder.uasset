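; Exploder enemy NPC Blueprint that detonates when it gets close to the player.
; Each tick while alive, it compares distance to the player against AttackRange.
; In range, it marks itself dead, disables capsule collision, spawns a scaled explosion particle and spawns a BP_Explosion_Hitbox actor at its location.
; Overlap and tick call the parent versions, while the parent BeginPlay call is disconnected.
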(event Collision|EventActorBeginOverlap
  (params (OtherActor :type Actor%20Object%20Reference))
  (|CallParentFunction OtherActor))

(event EventTick
  (params (DeltaSeconds :type Float%20%28single-precision%29))
  (|CallParentFunction DeltaSeconds)
  (if (Variables|Default|GetAlive)
    ;[1 1 1] Check if within attack radius of player
    (bind _distance (CallFunction|DistancetoPlayer))
    (bind _output_get (Variables|Default|SetAttack (<= _distance (Variables|Default|GetAttackRange))))
    (if _output_get
      (Variables|Default|SetAlive false)
      (Collision|SetCollisionEnabled (Variables|Default|GetCapsuleComponent) "NoCollision")
      (Effects|SpawnEmitteratLocation "/Game/StarterContent/Particles/P_Explosion.P_Explosion" (Transformation|GetActorLocation) "0, 0, 0" "1.500000,1.500000,1.500000")
      (Game|SpawnActorfromClass "/Game/NPCs/Exploder/BP_Explosion_Hitbox.BP_Explosion_Hitbox_C" (Math|Transform|MakeTransform (Transformation|GetActorLocation)) "Undefined" 0 0))))

(fn ConstructionScript
  (|CallParentFunction))