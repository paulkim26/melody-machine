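; BP_Brawler is a melee NPC that damages the player when within attack range.
; Each Tick, after the parent logic, a living brawler compares its distance to the player against AttackRange and sets the Attack flag.
; While in range, a windup timer accumulates delta time, calls TakeDamage on BP_Player at its maximum, then restarts.
; Leaving range also resets the windup.
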(event EventBeginPlay
  (|CallParentFunction) ; This node is disabled and will not be called.\nDrag off pins to build functionality.
)

(event Collision|EventActorBeginOverlap
  (params (OtherActor :type Actor%20Object%20Reference))
  (|CallParentFunction OtherActor))

(event EventTick
  (params (DeltaSeconds :type Float%20%28single-precision%29))
  (|CallParentFunction DeltaSeconds)
  (if (Variables|Default|GetAlive)
    ;[1 1 1] Check if within attack radius of player
    (bind _distance (CallFunction|DistancetoPlayer))
    (bind _output_get (Variables|Default|SetAttack (<= _distance (Variables|Default|GetAttackRange))))
    (if _output_get
      ;[1 1 1] Windup for attack
      (bind _output_get_2 (Variables|Default|SetWindup (+ (Variables|Default|GetWindup) (Utilities|Time|GetWorldDeltaSeconds))))
      (if (>= _output_get_2 (Variables|Default|GetWindupMax))
        ;[1 1 1] Inflict damage
        (bind _asbp_player (Utilities|Casting|CastToBP_Player (Game|Player|GetPlayerPawn 0)))
        (Default|TakeDamage _asbp_player)
        ;[1 1 1] Reset windup
        (Variables|Default|SetWindup 0.0 :!label _label))
      (else
        (goto _label)))))

(fn ConstructionScript
  (|CallParentFunction))