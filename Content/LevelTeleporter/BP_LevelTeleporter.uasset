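; BP_LevelTeleporter is a level-transition actor that opens the level named by its Level variable when the player pawn overlaps it.
; Every tick, AnimateArrow spins the Scene component and bobs it on a sine wave around its starting location, using a wrapped phase set by length and offset variables.
; Teleport's branch condition is hardwired true, so its "Can't open level" message never prints.
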(event EventBeginPlay
  (Variables|Default|SetOrigin (Transformation|GetWorldLocation (Variables|Default|GetScene))))

(event Collision|EventActorBeginOverlap
  (params (OtherActor :type Actor%20Object%20Reference))
  (if (== OtherActor (Game|Player|GetPlayerPawn 0))
    (CallFunction|Teleport)))

(event EventTick
  (params (DeltaSeconds :type Float%20%28single-precision%29))
  (CallFunction|AnimateArrow))

(fn ConstructionScript)

(fn AnimateArrow
  (bind _returnvalue (Utilities|Time|GetWorldDeltaSeconds))
  (bind _arrowanimationlength (Variables|Default|GetArrowAnimationLength))
  (bind _returnvalue_2 (/ _returnvalue _arrowanimationlength))
  (Variables|Default|SetArrowAnimationPhase (Math|Float|%(Float) (+ _returnvalue_2 (Variables|Default|GetArrowAnimationPhase)) 1.0))
  (Transformation|AddLocalRotation (Variables|Default|GetScene) (Math|Rotator|MakeRotator 0.0 0.0 (* _returnvalue_2 3.6e+02)) false false)
  (Transformation|SetWorldLocation (Variables|Default|GetScene) (+ (Variables|Default|GetOrigin) (Math|Vector|MakeVector 0.0 0.0 (* (Math|Trig|Sin(Degrees) (* (Variables|Default|GetArrowAnimationPhase) 3.6e+02)) (Variables|Default|GetArrowAnimationOffset)))) false false))

(fn Teleport
  (if true
    (Game|OpenLevel(byName) (Utilities|String|StringToName (Variables|Default|GetLevel)))
    (else
      (Development|PrintString (Utilities|String|Append "Can't open level \"" (Variables|Default|GetLevel) "\"")))))