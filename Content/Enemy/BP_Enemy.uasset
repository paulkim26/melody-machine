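; Enemy character that spawns as a random townsperson and walks continuously, with no targeting or attack logic.
; BeginPlay calls SetRandomSkin to pick one of 17 skeletal mesh slots (business shirt appears twice), applies it, then randomizes actor yaw.
; Tick adds movement input scaled by WalkSpeed along the control rotation's yaw, rather than reading the actor's rotation directly.
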(event EventBeginPlay
  ;[1 1 1] set random skin
  (CallFunction|SetRandomSkin)
  (Class|SkinnedMeshComponent|SetSkeletalMesh (Variables|Character|GetMesh) (Variables|Default|GetSkin) true)
  ;[1 1 1] set random initial direction
  (Transformation|SetActorRotation (Math|Rotator|MakeRotator 0.0 0.0 (Math|Random|RandomFloatinRange -1.8e+02 1.8e+02))))

(event Collision|EventActorBeginOverlap
  (params (OtherActor :type Actor%20Object%20Reference)))

(event EventTick
  (params (DeltaSeconds :type Float%20%28single-precision%29))
  ;[1 1 1] walk forward
  (Pawn|Input|AddMovementInput (Math|Vector|GetForwardVector (Math|Rotator|MakeRotator 0.0 0.0 (.Yaw (Math|Rotator|BreakRotator (Pawn|GetControlRotation :!class /Script/Engine.Pawn))))) (Variables|Default|GetWalkSpeed) false))

(fn ConstructionScript)

(fn SetRandomSkin
  (switch int (Math|Random|RandomInteger 17)
    (:0
      (Variables|Default|SetSkin "/Game/PolygonTown/Meshes/Characters/SK_Character_BusinessMan_Shirt.SK_Character_BusinessMan_Shirt"))
    (:1
      (Variables|Default|SetSkin "/Game/PolygonTown/Meshes/Characters/SK_Character_BusinessWoman.SK_Character_BusinessWoman"))
    (:2
      (Variables|Default|SetSkin "/Game/PolygonTown/Meshes/Characters/SK_Character_BusinessMan_Suit.SK_Character_BusinessMan_Suit"))
    (:3
      (Variables|Default|SetSkin "/Game/PolygonTown/Meshes/Characters/SK_Character_ShopKeeper.SK_Character_ShopKeeper"))
    (:4
      (Variables|Default|SetSkin "/Game/PolygonTown/Meshes/Characters/SK_Character_Father_01.SK_Character_Father_01"))
    (:5
      (Variables|Default|SetSkin "/Game/PolygonTown/Meshes/Characters/SK_Character_Father_02.SK_Character_Father_02"))
    (:6
      (Variables|Default|SetSkin "/Game/PolygonTown/Meshes/Characters/SK_Character_Female_Coat.SK_Character_Female_Coat"))
    (:7
      (Variables|Default|SetSkin "/Game/PolygonTown/Meshes/Characters/SK_Character_Female_Jacket.SK_Character_Female_Jacket"))
    (:8
      (Variables|Default|SetSkin "/Game/PolygonTown/Meshes/Characters/SK_Character_Female_Police.SK_Character_Female_Police"))
    (:9
      (Variables|Default|SetSkin "/Game/PolygonTown/Meshes/Characters/SK_Character_BusinessMan_Shirt.SK_Character_BusinessMan_Shirt"))
    (:10
      (Variables|Default|SetSkin "/Game/PolygonTown/Meshes/Characters/SK_Character_Male_Hoodie.SK_Character_Male_Hoodie"))
    (:11
      (Variables|Default|SetSkin "/Game/PolygonTown/Meshes/Characters/SK_Character_Male_Jacket.SK_Character_Male_Jacket"))
    (:12
      (Variables|Default|SetSkin "/Game/PolygonTown/Meshes/Characters/SK_Character_Male_Police.SK_Character_Male_Police"))
    (:13
      (Variables|Default|SetSkin "/Game/PolygonTown/Meshes/Characters/SK_Character_Mother.SK_Character_Mother"))
    (:14
      (Variables|Default|SetSkin "/Game/PolygonTown/Meshes/Characters/SK_Character_Mother_02.SK_Character_Mother_02"))
    (:15
      (Variables|Default|SetSkin "/Game/PolygonTown/Meshes/Characters/SK_Character_SchoolBoy.SK_Character_SchoolBoy"))
    (:16
      (Variables|Default|SetSkin "/Game/PolygonTown/Meshes/Characters/SK_Character_SchoolGirl.SK_Character_SchoolGirl"))))