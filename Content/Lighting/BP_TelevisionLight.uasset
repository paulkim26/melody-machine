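; Television prop that flickers its screen and the light it casts on and off at random.
; It starts off on BeginPlay, then Tick uses a short random Delay as an irregular timer to alternate between TurnOn and TurnOff.
; Each function sets the RectLight visibility, swaps the television's screen material between glowing and plain, and updates the ScreenOn flag that drives the next toggle.
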(event EventBeginPlay
  (CallFunction|TurnOff))

(event Collision|EventActorBeginOverlap
  (params (OtherActor :type Actor%20Object%20Reference)))

(event EventTick
  (params (DeltaSeconds :type Float%20%28single-precision%29))
  (Utilities|FlowControl|Delay (Math|Random|RandomFloatinRange 0.1 0.4))
  (if (Variables|Default|GetscreenOn)
    (CallFunction|TurnOff)
    (else
      (CallFunction|Turnon))))

(fn ConstructionScript)

(fn Turnon
  (Rendering|SetVisibility (Variables|Default|GetRectLight) true false)
  (Rendering|Material|SetMaterial (Variables|Default|GetTelevision) 1 "/Game/PolygonTown/Materials/Misc/Mat_TVScreenGlow.Mat_TVScreenGlow")
  (Variables|Default|SetscreenOn true))

(fn TurnOff
  (Rendering|SetVisibility (Variables|Default|GetRectLight) false false)
  (Rendering|Material|SetMaterial (Variables|Default|GetTelevision) 1 "/Game/PolygonTown/Materials/Misc/Mat_TVScreen.Mat_TVScreen")
  (Variables|Default|SetscreenOn false))