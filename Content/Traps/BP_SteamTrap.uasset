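; BP_SteamTrap is a steam trap that damages the player for as long as they stay in its Steam component.
; Overlap sets PlayerInRadius and starts a delayed loop that drains BP_Player Health until the overlap ends or health runs out, when it calls JumpToSafeLocation on the player pawn.
; A custom event, not called here, sets a looping timer for a "Sphere" function that this file does not define.
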(event OnComponentBeginOverlap(Steam)
  (params (OverlappedComponent :type Primitive%20Component%20Object%20Reference) (OtherActor :type Actor%20Object%20Reference) (OtherComp :type Primitive%20Component%20Object%20Reference) (OtherBodyIndex :type Integer) (bFromSweep :type Boolean) (SweepResult :type Hit%20Result%20Structure%20%28by%20ref%29))
  (bind _asbp_player (Utilities|Casting|CastToBP_Player OtherActor))
  (Variables|Default|SetPlayerInRadius true)
  (bind _output_get (Variables|/Game/Player/BP_Player.BP_Player_C|SetHealth _asbp_player (- (Variables|/Game/Player/BP_Player.BP_Player_C|GetHealth _asbp_player) 1) :!label _label))
  (if (<= _output_get 0)
    (bind _asbp_player_2 (Utilities|Casting|CastToBP_Player (Game|Player|GetPlayerPawn 0)))
    (Default|JumptoSafeLocation _asbp_player_2)
    (else
      (Utilities|FlowControl|Delay 1.0)
      (if (Variables|Default|GetPlayerInRadius)
        (goto _label)))))

(event OnComponentEndOverlap(Steam)
  (params (OverlappedComponent :type Primitive%20Component%20Object%20Reference) (OtherActor :type Actor%20Object%20Reference) (OtherComp :type Primitive%20Component%20Object%20Reference) (OtherBodyIndex :type Integer))
  (Utilities|Casting|CastToBP_Player OtherActor)
  (Variables|Default|SetPlayerInRadius false))

(event Custom|CustomEvent
  (Utilities|Time|SetTimerbyFunctionName 0 "Sphere" 5.0 true))

(event Collision|EventActorBeginOverlap
  (params (OtherActor :type Actor%20Object%20Reference)))

(event EventTick
  (params (DeltaSeconds :type Float%20%28single-precision%29)))

(event EventBeginPlay)

(fn ConstructionScript)